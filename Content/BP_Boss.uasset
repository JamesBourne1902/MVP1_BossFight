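; Boss actor with a health bar, damageable only while the player stands on its head; death shows the win screen.
; Pooled enemy spawners appear at six points on start and after each jump attack.
; RaiseSteps builds a three-stage climb, delaying then disabling the timed jump, which launches a player off the head and resets the steps.
; At half health, a second timer spawns BP_CrazyCube projectiles from player-relative points.
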(event `self.ReceiveBeginPlay`
  ;[1 1 1] Sets up the boss health bar onto the player's screen
  (bind _returnvalue (`|CreateWidget` "/Game/Widgets/WB_BossHealthBar.WB_BossHealthBar_C"))
  (set `/Game/Widgets/WB_BossHealthBar.BossRef` self _returnvalue)
  (`UserWidget.AddToViewport` _returnvalue 0)
  ;[1 1 1] Populates the object pool for the enmy spawners
  (`/Game/AC_ObjectPool.PopulatePool` (`self.AC_ObjectPool`) (`self.SpawnPosList`) self)
  (`self.SummonPedastals`))

(event `self.HeadCollider.OnComponentBeginOverlap`
  (params (OverlappedComponent :type "PrimitiveComponent Object Reference") (OtherActor :type "Actor Object Reference") (OtherComp :type "PrimitiveComponent Object Reference") (OtherBodyIndex :type Integer) (bFromSweep :type Boolean) (SweepResult :type "HitResult Structure (by ref)"))
  ;[1 1 1] Collision logic:
  ; can take damage if player is inside collision box
  (if (== OtherActor (`GameplayStatics.GetPlayerCharacter` 0))
    (set `self.CanTakeDamage` true)
    ;[1 1 1] Gives the player a few seconds to attack the boss before being thrown off
    (set `self.JumpTimer` 22.0)
    (set `self.CanPerformJump` true)))

(event `self.BodyCollider.OnComponentBeginOverlap`
  (params (OverlappedComponent :type "PrimitiveComponent Object Reference") (OtherActor :type "Actor Object Reference") (OtherComp :type "PrimitiveComponent Object Reference") (OtherBodyIndex :type Integer) (bFromSweep :type Boolean) (SweepResult :type "HitResult Structure (by ref)"))
  (bind _returnvalue (`GameplayStatics.GetPlayerCharacter` 0))
  ;[1 1 1] Collision logic:
  ; Kills the player if they are jumped on
  (if (== OtherActor _returnvalue)
    (message `/Game/BPI_Damageable.Damageable` _returnvalue 500000.0)))

(event `self.HeadCollider.OnComponentEndOverlap`
  (params (OverlappedComponent :type "PrimitiveComponent Object Reference") (OtherActor :type "Actor Object Reference") (OtherComp :type "PrimitiveComponent Object Reference") (OtherBodyIndex :type Integer))
  ;[1 1 1] Collision logic:
  ; can take damage if player is inside collision box
  (if (== OtherActor (`GameplayStatics.GetPlayerCharacter` 0))
    (set `self.CanTakeDamage` false)
    ;[1 1 1] stops a second overlap when the player is sent flying from setting the jump timer (above)
    (if (== (`self.StepStage`) 0)
      (set `self.JumpTimer` 0.0))))

(event `/Game/BPI_Damageable.Damageable`
  (params (Damage :type "Float (double-precision)"))
  ;[1 1 1] Triggered when the player attacks this actor
  (`self.Apply Damage` Damage))

(event `MoveSteps1`
  (params (StepToMove :type "SceneComponent Object Reference") (NewPos :type "Vector Structure"))
  (bind _returnvalue_location (`KismetMathLibrary.BreakTransform` (`SceneComponent.GetRelativeTransform` StepToMove)))
  ;[1 1 1] Animates the rise and fall of the steps up to the boss head
  (bind (_direction _raisesteps) (`Timeline|StepRaise Timeline` :!via `PlayFromStart`)
    (:`Update`
      (`SceneComponent.K2_SetRelativeLocation` StepToMove (`KismetMathLibrary.VLerp` _returnvalue_location NewPos _raisesteps) false false))))

(event `MoveSteps2`
  (params (StepToMove :type "SceneComponent Object Reference") (NewPos :type "Vector Structure"))
  (bind _returnvalue_location (`KismetMathLibrary.BreakTransform` (`SceneComponent.GetRelativeTransform` StepToMove)))
  ;[1 1 1] Animates the rise and fall of the steps up to the boss head
  (bind (_direction _raisesteps) (`Timeline|Timeline` :!via `PlayFromStart`)
    (:`Update`
      (`SceneComponent.K2_SetRelativeLocation` StepToMove (`KismetMathLibrary.VLerp` _returnvalue_location NewPos _raisesteps) false false))))

(event `MoveSteps3`
  (params (StepToMove :type "SceneComponent Object Reference") (NewPos :type "Vector Structure"))
  (bind _returnvalue_location (`KismetMathLibrary.BreakTransform` (`SceneComponent.GetRelativeTransform` StepToMove)))
  ;[1 1 1] Animates the rise and fall of the steps up to the boss head
  (bind (_direction _raisesteps) (`Timeline|Timeline_0` :!via `PlayFromStart`)
    (:`Update`
      (`SceneComponent.K2_SetRelativeLocation` StepToMove (`KismetMathLibrary.VLerp` _returnvalue_location NewPos _raisesteps) false false))))

(event `JumpAttackAnimation`
  (bind _head (`self.Head`))
  (bind _originalbosspos (`self.OriginalBossPos`))
  ;[1 1 1] Animates the jump attack for the boss
  ; when the animation finishes a function to lower the steps is called
  (set `self.OriginalBossPos` (`SceneComponent.RelativeLocation` _head))
  (bind (_direction _newtrack_0) (`Timeline|JumpAttackTimeline` :!via `PlayFromStart`)
    (:`Update`
      (`SceneComponent.K2_SetRelativeLocation` _head (`KismetMathLibrary.VLerp` _originalbosspos (+ _originalbosspos (0.0 0.0 1000.0)) _newtrack_0) false false))
    (:`Finished`
      (`self.LowerSteps`)
      (`self.SummonPedastals`)
      (set `self.CanPerformJump` true))))

(event `self.ReceiveTick`
  (params (DeltaSeconds :type "Float (single-precision)"))
  ;[1 1 1] Every tick the timers are incremented by delta time
  ; One Timer controls the jump attack
  ; The other controls the projectile attack
  (`|ExecutionSequence`
    (:`then_0`
      (if (`self.CanPerformJump`)
        (bind _timerexceedsthreshold (`self.IncrementTimer` (`self.JumpTimer`) (`self.JumpDelayThreshold`)))
        (if _timerexceedsthreshold
          (`self.PerformJumpAttack`))))
    (:`then_1`
      (if (`self.AtStageTwo`)
        (bind _timerexceedsthreshold_2 (`self.IncrementTimer` (`self.ProjTimer`) (`self.ProjTimeThreshold`)))
        (if _timerexceedsthreshold_2
          (`self.SpawnProjectile`))))))

(fn `Apply Damage`
  (params (Damage :type "Float (double-precision)"))
  (if (`self.CanTakeDamage`)
    (bind _output_get (set `self.Health` (- (`self.Health`) Damage)))
    ;[1 1 1] If health is at 50%, AtStageTwo is set to true
    (set `self.AtStageTwo` (<= _output_get (/ (`self.MaxHealth`) 2.0)))
    (`self.CheckForDeath`)))

(fn `CheckForDeath`
  (if (<= (`self.Health`) 0.0)
    (`self.K2_DestroyActor`)
    (bind _returnvalue (`|CreateWidget` "/Game/Widgets/WB_WinScreen.WB_WinScreen_C" (`GameplayStatics.GetPlayerController` 0)))
    (`UserWidget.AddToViewport` _returnvalue 0)))

(fn `IncrementStepsCount`
  (set `self.StepStage` (`KismetMathLibrary.Clamp` (+ (`self.StepStage`) 1) 0 3)))

(fn `IncrementTimer`
  (params (Timer :type "Float (double-precision) (by ref)") (TimerThreshold :type "Float (double-precision)"))
  (returns (TimerExceedsThreshold :type Boolean))
  (bind _returnvalue (+ Timer (`GameplayStatics.GetWorldDeltaSeconds`)))
  (bind _returnvalue_2 (>= _returnvalue TimerThreshold))
  (if _returnvalue_2
    (`|VariableSetRef` Timer)
    (else
      (`|VariableSetRef` Timer _returnvalue)))
  (return _returnvalue_2))

(fn `LowerSteps`
  (bind _stepstage (`self.StepStage`))
  (if (== _stepstage 1)
    (`self.MoveSteps1` (`self.Step1`) (2320.0 3320.0 -1000.0))
    (set `self.StepStage` 0 :!label _label)
    (elif (== _stepstage 2)
      (`self.MoveSteps2` (`self.Step2`))
      (`self.MoveSteps1` (`self.Step1`) (2320.0 3320.0 -1000.0))
      (goto _label)
      (elif (== _stepstage 3)
        (`self.MoveSteps3` (`self.Step3`))
        (`self.MoveSteps2` (`self.Step2`))
        (`self.MoveSteps1` (`self.Step1`) (2320.0 3320.0 -1000.0))
        (goto _label)))))

(fn `PerformJumpAttack`
  (bind _returnvalue (`GameplayStatics.GetPlayerCharacter` 0))
  (set `self.CanPerformJump` false)
  (if (`self.CanTakeDamage`)
    (`Character.LaunchCharacter` _returnvalue (* (`KismetMathLibrary.MakeVector` (.x (`KismetMathLibrary.Normal` (- (`SceneComponent.K2_GetComponentLocation` (`Character.CapsuleComponent` _returnvalue)) (`SceneComponent.K2_GetComponentLocation` (`self.HeadCollider`))))) (.y (`KismetMathLibrary.Normal` (- (`SceneComponent.K2_GetComponentLocation` (`Character.CapsuleComponent` _returnvalue)) (`SceneComponent.K2_GetComponentLocation` (`self.HeadCollider`))))) 1.0) 2000.0) true true)
    (`self.JumpAttackAnimation`)
    (else
      (`self.JumpAttackAnimation`))))

(fn `RaiseSteps`
  (bind _stepstage (`self.StepStage`))
  (if (== _stepstage 0)
    (`self.IncrementStepsCount`)
    (`self.MoveSteps1` (`self.Step1`) (2320.0 3320.0 0.0))
    ;[1 1 1] Raising the first 2 steps give a 10 second delay to the bosses jump
    (set `self.JumpTimer` (- (`self.JumpTimer`) 10.0) :!label _label)
    (elif (== _stepstage 1)
      (`self.IncrementStepsCount`)
      (`self.MoveSteps2` (`self.Step2`) (-94.0 0.0 94.0))
      (goto _label)
      (elif (== _stepstage 2)
        (`self.IncrementStepsCount`)
        (`self.MoveSteps3` (`self.Step3`) (-94.0 0.0 94.0))
        ;[1 1 1] Raising the last step disables the bosses jump (this is to prevent unfair timings)
        (set `self.CanPerformJump` false)))))

(fn `SpawnProjectile`
  (bind _x (.x (`KismetMathLibrary.InverseTransformLocation` (`SceneComponent.K2_GetComponentToWorld` (`self.Body`)) (`self.K2_GetActorLocation` (`GameplayStatics.GetPlayerCharacter` 0)))))
  (bind _y (.y (`KismetMathLibrary.InverseTransformLocation` (`SceneComponent.K2_GetComponentToWorld` (`self.Body`)) (`self.K2_GetActorLocation` (`GameplayStatics.GetPlayerCharacter` 0)))))
  (if (> (`KismetMathLibrary.Abs` _x) (`KismetMathLibrary.Abs` _y))
    (if (> _x 0.0)
      (set `self.ProjSpawnPoint` (`SceneComponent.K2_GetComponentLocation` (`self.ProjSpawn+X>Z`)))
      (else
        (set `self.ProjSpawnPoint` (`SceneComponent.K2_GetComponentLocation` (`self.ProjSpawn-X>Z`)))))
    (elif (> _y 0.0)
      (set `self.ProjSpawnPoint` (`SceneComponent.K2_GetComponentLocation` (`self.ProjSpawn+Z>X`)))
      (else
        (set `self.ProjSpawnPoint` (`SceneComponent.K2_GetComponentLocation` (`self.ProjSpawn-Z>X`))))))
  (`|SpawnActorFromClass` "/Game/BP_CrazyCube.BP_CrazyCube_C" (`KismetMathLibrary.MakeTransform` (`self.ProjSpawnPoint`)) "Undefined" "MultiplyWithRoot" null null))

(fn `SummonPedastals`
  (for _ (`self.SpawnPosList`)
    (if true
      (bind _actorspawned (`/Game/AC_ObjectPool.SpawnActorFromPool` (`self.AC_ObjectPool`)))
      (bind _asbp_enemy_spawner (cast `/Game/BP_EnemySpawner` _actorspawned))
      (`/Game/BP_EnemySpawner.SpawnEnemyActor` _asbp_enemy_spawner)
      (else
        (break)))))

(fn `UserConstructionScript`
  (bind _spawnposlist (`self.SpawnPosList`))
  (set `self.MaxHealth` (`self.Health`))
  ;[1 1 1] Adds the spawn positions for the pedastals to an array
  (`KismetArrayLibrary.Array_Add` _spawnposlist (`SceneComponent.K2_GetComponentLocation` (`self.Point6`)))
  (`KismetArrayLibrary.Array_Add` _spawnposlist (`SceneComponent.K2_GetComponentLocation` (`self.Point5`)))
  (`KismetArrayLibrary.Array_Add` _spawnposlist (`SceneComponent.K2_GetComponentLocation` (`self.Point4`)))
  (`KismetArrayLibrary.Array_Add` _spawnposlist (`SceneComponent.K2_GetComponentLocation` (`self.Point3`)))
  (`KismetArrayLibrary.Array_Add` _spawnposlist (`SceneComponent.K2_GetComponentLocation` (`self.Point2`)))
  (`KismetArrayLibrary.Array_Add` _spawnposlist (`SceneComponent.K2_GetComponentLocation` (`self.Point1`))))