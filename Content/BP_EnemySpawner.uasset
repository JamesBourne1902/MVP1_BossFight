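; Destructible enemy spawner that spawns an enemy at its spawn point on a repeating interval.
; Tick accumulates a timer and calls SpawnEnemy with the spawn point's world location.
; Damage from the Damageable event lowers Health; at zero the spawner returns to a pool, restores the Health cached at construction, and calls RaiseSteps on a linked boss if valid.
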(event `self.ReceiveTick`
  (params (DeltaSeconds :type "Float (single-precision)"))
  ;[1 1 1] Periodically spawns an enemy on its spawn point
  (bind _output_get (set `self.Timer` (+ DeltaSeconds (`self.Timer`))))
  (if (>= _output_get (`self.SpawnInterval`))
    (`self.SpawnEnemyActor`)
    (set `self.Timer` 0.0)))

(event `/Game/BPI_Damageable.Damageable`
  (params (Damage :type "Float (double-precision)"))
  ;[1 1 1] Event triggered when attacked by the player.
  ; applies damage to this actor
  (set `self.Health` (- (`self.Health`) Damage))
  (`self.CheckForDeath`))

(fn `CheckForDeath`
  (bind _bossref (`self.BossRef`))
  (if (<= (`self.Health`) 0.0)
    (`self.ReturnToPool`)
    (set `self.Health` (`self.MaxHealth`))
    (if (`KismetSystemLibrary.IsValid` _bossref)
      (`/Game/BP_Boss.RaiseSteps` _bossref))))

(fn `SpawnEnemyActor`
  (`/Game/BPFL_FunctionLibrary.Spawn Enemy` (`SceneComponent.K2_GetComponentLocation` (`self.SpawnPoint`))))

(fn `UserConstructionScript`
  (set `self.MaxHealth` (`self.Health`)))