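; A melee enemy that damages the first-person player when within range, takes damage through Damageable, and destroys itself at zero health.
; Tick turns its health bar widget toward the camera and polls player distance, triggering cooldown-gated attacks animated by a timeline rotating the body.
; On construction it checks whether BP_Boss is at stage two, and if so tilts the eyes and sets a different attack damage.
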(event `/Game/BPI_Damageable.Damageable`
  (params (Damage :type "Float (double-precision)"))
  ;[1 1 1] Event triggered when attacked by the player
  (`self.ApplyDamage` Damage)
  (`self.UpdateHealthBar`)
  (`self.DeathCheck`))

(event `self.ReceiveTick`
  (params (DeltaSeconds :type "Float (single-precision)"))
  ;[1 1 1] Every frame:
  ; Rotates the enemy health bar to face the player camera
  (`self.RotateHealthBar`)
  ;[1 1 1] Every frame:
  ; finds the distance between the enemy and the player
  ; If its within the threshhold, attack the player
  (bind _dist (`self.CalculateDistToPlayer`))
  (if (<= _dist (`self.MinAttackDistThreshhold`))
    (`self.AttemptAttack`)))

(event `AttackCooldown`
  ;[1 1 1] Resets the attack after the given cooldown length
  (`KismetSystemLibrary.Delay` (`self.AttackCooldownLength`))
  (set `self.AttackOnCooldown` false))

(event `AnimateAttack`
  ;[1 1 1] Rotates the body.
  ; used to represent an attack animation
  (bind (_direction _rotation_track) (`Timeline|Animate Timeline` :!via `PlayFromStart`)
    (:`Update`
      (`SceneComponent.K2_SetRelativeRotation` (`self.body`) (`KismetMathLibrary.RLerp` (struct) (struct :`Pitch` -90.0) _rotation_track) false false))))

(fn `ApplyDamage`
  (params (Damage :type "Float (double-precision)"))
  (set `self.Health` (- (`self.Health`) Damage)))

(fn `AttemptAttack`
  (if (not (`self.AttackOnCooldown`))
    (set `self.AttackOnCooldown` true)
    (`self.AttackCooldown`)
    (bind _asbp_first_person_character (cast `/Game/FirstPerson/Blueprints/BP_FirstPersonCharacter` (`GameplayStatics.GetPlayerCharacter` 0)))
    (`/Game/BPI_Damageable.Damageable` _asbp_first_person_character (`self.AttackDamage`))
    (`self.AnimateAttack`)))

(fn `CalculateDistToPlayer`
  (returns (Dist :type "Float (double-precision)"))
  (return (`KismetMathLibrary.VSize` (- (`self.K2_GetActorLocation` (`GameplayStatics.GetPlayerCharacter` 0)) (`SceneComponent.K2_GetComponentLocation` (`self.CapsuleComponent`))))))

(fn `DeathCheck`
  (if (<= (`self.Health`) 0.0)
    (`self.K2_DestroyActor`)))

(fn `RotateHealthBar`
  (bind _health_bar (`self.Health Bar`))
  (`SceneComponent.K2_SetWorldRotation` _health_bar (`KismetMathLibrary.FindLookAtRotation` (`KismetMathLibrary.MakeVector` (.x (`SceneComponent.K2_GetComponentLocation` _health_bar)) (.y (`SceneComponent.K2_GetComponentLocation` _health_bar))) (`KismetMathLibrary.MakeVector` (.x (`SceneComponent.K2_GetComponentLocation` (`PlayerCameraManager.TransformComponent` (`GameplayStatics.GetPlayerCameraManager` 0)))) (.y (`SceneComponent.K2_GetComponentLocation` (`PlayerCameraManager.TransformComponent` (`GameplayStatics.GetPlayerCameraManager` 0)))))) false false))

(fn `UpdateHealthBar`
  (bind _aswb_health_bar (cast `/Game/Widgets/WB_HealthBar` (`WidgetComponent.GetWidget` (`self.Health Bar`))))
  (`ProgressBar.SetPercent` (`/Game/Widgets/WB_HealthBar.HealthBar` _aswb_health_bar) (/ (`self.Health`) (`self.MaxHealth`))))

(fn `UserConstructionScript`
  (set `self.MaxHealth` (`self.Health`))
  (bind _returnvalue (`GameplayStatics.GetActorOfClass` "/Game/BP_Boss.BP_Boss_C"))
  (if (`/Game/BP_Boss.AtStageTwo` _returnvalue)
    (`SceneComponent.K2_SetRelativeRotation` (`self.left eye`) (struct :`Roll` -30.0) false false)
    (`SceneComponent.K2_SetRelativeRotation` (`self.Right eye`) (struct :`Roll` 30.0) false false)
    (set `self.AttackDamage` 7.5)))