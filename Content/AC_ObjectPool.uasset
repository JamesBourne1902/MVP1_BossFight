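; Object pool component that pre-spawns and recycles actors, set up for enemy spawners used by a boss.
; PopulatePool spawns one actor per supplied position, casts it to BP_EnemySpawner to pass the boss reference, then stores it and returns it to the pool.
; SpawnActorFromPool takes out the first actor flagged as in the pool, found by linear search, and never spawns extras when none are free.
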(event `PopulatePool`
  (params (SpawnPosArray :type "Array of Vector Structure") (BossRef :type "/Game/BP_Boss Object Reference"))
  ;[1 1 1] Populates the pool on start up
  (for _array_element SpawnPosArray
    (bind _returnvalue (`|SpawnActorFromClass` (`self.PooledActorClassRef`) (`KismetMathLibrary.MakeTransform` _array_element) "Undefined" "MultiplyWithRoot" null null))
    (bind _asbp_enemy_spawner (cast `/Game/BP_EnemySpawner` _returnvalue))
    (set `/Game/BP_EnemySpawner.BossRef` BossRef _asbp_enemy_spawner)
    (`KismetArrayLibrary.Array_AddUnique` (`self.ObjectPool`) _returnvalue)
    (`/Game/BP_PooledActor.ReturnToPool` _returnvalue)))

(fn `Retrieve Actor from Pool`
  (returns (PooledObject :type "/Game/BP_PooledActor Object Reference"))
  (for _array_element (`self.ObjectPool`)
    (if (`/Game/BP_PooledActor.ActorInPool` _array_element)
      (return _array_element))))

(fn `SpawnActorFromPool`
  (returns (ActorSpawned :type "/Game/BP_PooledActor Object Reference"))
  (bind _pooledobject (`self.Retrieve Actor from Pool`))
  (`/Engine/EditorBlueprintResources/StandardMacros.IsValid` _pooledobject
    (:`Is Valid`
      (`/Game/BP_PooledActor.TakeFromPool` _pooledobject)
      (return _pooledobject))))