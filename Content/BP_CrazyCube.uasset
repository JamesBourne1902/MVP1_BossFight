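; Crazy cube projectile that tumbles through random rotations, then homes in on the player.
; A looping timeline lerps between target rotations, switching to look-at rotations toward the player camera once the random spin count reaches its maximum.
; After a short delay, Tick moves it along its forward vector without sweep, re-aiming each timeline cycle.
; Overlapping the player deals damage and destroys it, as does being attacked through the Damageable event.
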(event `self.ReceiveBeginPlay`
  ;[1 1 1] Starts the cube spinning when it spawns in
  (`self.RandomRotation`))

(event `RandomRotation`
  ;[1 1 1] Spins the cube in a random frantic motion
  (`self.SetTargetRotation`)
  (bind (_direction _newtrack_0) (`Timeline|RotationTimeLine` :!via `PlayFromStart`)
    (:`Update`
      (`SceneComponent.K2_SetRelativeRotation` (`self.Projectile`) (`KismetMathLibrary.RLerp` (`self.OldRotation`) (`self.TargetRotation`) _newtrack_0) false false))
    (:`Finished`
      (`self.IncrementRotationCounter`)
      (`self.RandomRotation`))))

(event `self.ReceiveTick`
  (params (DeltaSeconds :type "Float (single-precision)"))
  ;[1 1 1] Applies a constant forward velocity to the projectile
  (if (`self.CanMove`)
    (`self.MoveProjectile` (`SceneComponent.GetForwardVector` (`self.Projectile`)) (`self.ForwardVelocity`))))

(event `UpdateMoveable`
  ;[1 1 1] Sets the 'canMove' bool to true
  (`KismetSystemLibrary.Delay` 0.5)
  (set `self.CanMove` true))

(event `self.Collider.OnComponentBeginOverlap`
  (params (OverlappedComponent :type "PrimitiveComponent Object Reference") (OtherActor :type "Actor Object Reference") (OtherComp :type "PrimitiveComponent Object Reference") (OtherBodyIndex :type Integer) (bFromSweep :type Boolean) (SweepResult :type "HitResult Structure (by ref)"))
  ;[1 1 1] Triggered when the player is hit with this projectile
  (if (== OtherActor (`GameplayStatics.GetPlayerCharacter` 0))
    (message `/Game/BPI_Damageable.Damageable` OtherActor 20.0)
    (`self.K2_DestroyActor`)))

(event `/Game/BPI_Damageable.Damageable`
  (params (Damage :type "Float (double-precision)"))
  ;[1 1 1] Triggered when the player attacks this actor.
  ; Destroys the actor
  (`self.K2_DestroyActor`))

(fn `IncrementRotationCounter`
  (set `self.OldRotation` (`self.TargetRotation`))
  (set `self.RotationCounter` (+ (`self.RotationCounter`) 1)))

(fn `MoveProjectile`
  (params (Dir :type "Vector Structure") (velocity :type "Float (double-precision)"))
  (`SceneComponent.K2_SetWorldLocation` (`self.Projectile`) (+ (* Dir velocity (`GameplayStatics.GetWorldDeltaSeconds`)) (`SceneComponent.K2_GetComponentLocation` (`self.Projectile`))) false false))

(fn `SetTargetRotation`
  (if (< (`self.RotationCounter`) (`self.MaxRandomRotations`))
    (set `self.TargetRotation` (`KismetMathLibrary.RandomRotator` false))
    (else
      (set `self.TargetRotation` (`KismetMathLibrary.FindLookAtRotation` (`SceneComponent.K2_GetComponentLocation` (`self.Projectile`)) (`SceneComponent.K2_GetComponentLocation` (`PlayerCameraManager.TransformComponent` (`GameplayStatics.GetPlayerCameraManager` 0)))))
      (if (not (`self.CanMove`))
        (`self.UpdateMoveable`)))))

(fn `UserConstructionScript`)